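; AI controller for LightWars that acts as the engine-side view of a separate LightWarsController object, constructed with the game mode on BeginPlay.
; It forwards Tick and generator zone enter/exit events to that object.
; As a PlayerObserver, it tints the pawn's mesh to the team color through a dynamic material instance, while UpdateLight is empty.
; Its only movement is a constant slow push along world +X each frame.
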(event `self.ReceiveBeginPlay`
  (`KismetSystemLibrary.PrintString` "AIController Init running")
  (bind _aslight_wars_game_mode (cast `/Game/LightWarsBP/Blueprints/UE4Controller/LightWarsGameMode` (`GameplayStatics.GetGameMode`)))
  (bind _returnvalue (`|GenericCreateObject` "/Game/LightWarsBP/Blueprints/UE4Controller/LightWarsController.LightWarsController_C" self _aslight_wars_game_mode))
  (bind _output_get (set `self.Controller` _returnvalue))
  (`/Game/LightWarsBP/Blueprints/UE4Controller/LightWarsController.Init` _output_get self)
  (`KismetSystemLibrary.PrintString` "AIController Init Success"))

(event `self.ReceiveTick`
  (params (DeltaSeconds :type "Float (single-precision)"))
  (`/Game/LightWarsBP/Blueprints/UE4Controller/LightWarsController.Tick` (`self.Controller`) DeltaSeconds)
  (bind _ascharacter (cast `Character` (`self.K2_GetPawn`)))
  (`Pawn.AddMovementInput` _ascharacter (1.0 0.0 0.0) 0.1 false))

(event `/Game/LightWarsBP/Blueprints/Model/PlayerObserver.UpdateLight`
  (params (Light :type "Float (single-precision)"))
  ;[1 1 1] PlayerObserver
)

(event `/Game/LightWarsBP/Blueprints/Model/PlayerObserver.UpdateTeam`
  (params (Team :type "/Game/LightWarsBP/Blueprints/Model/Team Object Reference"))
  ;[1 1 1] PlayerObserver
  (bind _aslight_wars_character (cast `/Game/LightWarsBP/Blueprints/UE4View/LightWarsCharacter` (`self.K2_GetPawn`)))
  (bind _returnvalue (`KismetMaterialLibrary.CreateDynamicMaterialInstance` "/Game/Mannequin/Character/Materials/M_UE4Man_BodyInstance.M_UE4Man_BodyInstance"))
  (`MaterialInstanceDynamic.SetVectorParameterValue` _returnvalue "BodyColor" (`/Game/LightWarsBP/Blueprints/Model/Team.Color` Team))
  (`PrimitiveComponent.SetMaterial` (`Character.Mesh` _aslight_wars_character) 0 _returnvalue))

(event `EnterZone`
  (params (Generator :type "/Game/LightWarsBP/Blueprints/Model/Generator Object Reference"))
  (`/Game/LightWarsBP/Blueprints/UE4Controller/LightWarsController.EnterZone` (`self.Controller`) Generator))

(event `ExitZone`
  (params (Generator :type "/Game/LightWarsBP/Blueprints/Model/Generator Object Reference"))
  (`/Game/LightWarsBP/Blueprints/UE4Controller/LightWarsController.ExitZone` (`self.Controller`) Generator))

(fn `UserConstructionScript`)
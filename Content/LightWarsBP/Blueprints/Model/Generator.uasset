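; Capturable generator that teams take over by having more players turning it on than rival teams.
; Turn-on events maintain per-team player counts, picking a leading team and its margin, which FindDifference caps at the array length.
; Tick scales capture progress by that margin, draining a previous team's progress to neutral before building the new one's, and decays unowned progress when empty.
; TeamOwner's OnRep notifies an Observer of ownership changes.
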(event Custom|StopTurnOn
  (params (Player :type Light%20Wars%20Player%20Object%20Reference))
  (Utilities|Array|RemoveItem (Variables|Algo|GetPlayers) Player)
  (CallFunction|RemoveTeam (Variables|/Game/LightWarsBP/Blueprints/Model/LightWarsPlayer.LightWarsPlayer_C|GetTeamOwner Player)))

(event Custom|AddTeam
  (params (Team :type Team%20Object%20Reference))
  (bind _teams (Variables|Algo|GetTeams))
  (bind _playersbyteam (Variables|Algo|GetPlayersByTeam))
  (bind _returnvalue (Utilities|Array|FindItem _teams Team))
  (if (Utilities|Array|ContainsItem (Variables|Algo|GetTeams) Team)
    _
    (else
      (Utilities|Array|AddUnique (Variables|Algo|GetTeams) Team)))
  (Utilities|Array|SetArrayElem _playersbyteam _returnvalue (+ (Utilities|Array|Get(acopy) _playersbyteam _returnvalue) 1) true)
  (CallFunction|UpdateWinningTeam))

(event Custom|RemoveTeam
  (params (Team :type Team%20Object%20Reference))
  (bind _teams (Variables|Algo|GetTeams))
  (bind _playersbyteam (Variables|Algo|GetPlayersByTeam))
  (bind _returnvalue (Utilities|Array|FindItem _teams Team))
  (Utilities|Array|SetArrayElem _playersbyteam _returnvalue (- (Utilities|Array|Get(acopy) _playersbyteam _returnvalue) 1))
  (CallFunction|UpdateWinningTeam))

(event Custom|Tick
  (params (Delta :type Float%20%28single-precision%29))
  (bind _advantagewinningteam (Variables|Algo|GetAdvantageWinningTeam))
  (bind _factor_time (Variables|Default|GetFACTOR_TIME))
  (bind _returnvalue (Math|Conversions|ToFloat(Integer) _advantagewinningteam))
  (bind _returnvalue_2 (* Delta _returnvalue _factor_time))
  (Utilities|FlowControl|Sequence
    (:then_0
      (if (and (== (Variables|Algo|GetPreviousWinningTeam) 0) (!= (Variables|Algo|GetCurrentWinningTeam) 0))
        (Variables|Algo|SetPreviousWinningTeam (Variables|Algo|GetCurrentWinningTeam))))
    (:then_1
      (if (!= (Variables|Algo|GetCurrentWinningTeam) 0)
        (if (== (Variables|Algo|GetCurrentWinningTeam) (Variables|Algo|GetPreviousWinningTeam))
          (bind _output_get (Variables|Default|SetProgressCapture (+ _returnvalue_2 (Variables|Default|GetProgressCapture))))
          (if (>= _output_get (Variables|Default|GetPROGRESS100))
            (Variables|Default|SetProgressCapture (Variables|Default|GetPROGRESS100))
            (if (!= (Variables|Default|GetTeamOwner) (Variables|Algo|GetCurrentWinningTeam))
              (Variables|Default|SetTeamOwner (Variables|Algo|GetCurrentWinningTeam))))
          (else
            (bind _output_get_2 (Variables|Default|SetProgressCapture (- (Variables|Default|GetProgressCapture) _returnvalue_2)))
            (if (<= _output_get_2 0.0)
              (Variables|Algo|SetPreviousWinningTeam (Variables|Algo|GetCurrentWinningTeam))
              (Variables|Default|SetProgressCapture (Math|Float|Absolute(Float) (Variables|Default|GetProgressCapture)))
              (Variables|Default|SetTeamOwner 0))))
        (elif (not (!= (Variables|Default|GetTeamOwner) 0))
          (bind _output_get_3 (Variables|Default|SetProgressCapture (- (Variables|Default|GetProgressCapture) (* Delta (Variables|Default|GetFACTOR_TIME)))))
          (if (<= _output_get_3 0.0)
            (Variables|Default|SetProgressCapture 0.0)
            (Variables|Algo|SetPreviousWinningTeam 0)))))))

(event Custom|PrintState
  (Development|PrintString 0 "----------")
  (for (_array_element _array_index) (Variables|Algo|GetTeams)
    (Development|PrintString 0 (Utilities|String|ToString(Integer) (Variables|/Game/LightWarsBP/Blueprints/Model/Team.Team_C|GetColor _array_element)))
    (Development|PrintString 0 (Utilities|String|ToString(Integer) (Utilities|Array|Get(acopy) (Variables|Algo|GetPlayersByTeam) _array_index)))
    (Development|PrintString 0 "next")))

(event Custom|UpdateWinningTeam
  (bind _playersbyteam (Variables|Algo|GetPlayersByTeam))
  (bind (_indexofmaxvalue _maxvalue) (Math|Integer|MaxOfIntArray _playersbyteam))
  (if (> _maxvalue 0)
    (Variables|Algo|SetCurrentWinningTeam (Utilities|Array|Get(acopy) (Variables|Algo|GetTeams) _indexofmaxvalue))
    (bind _difference (CallFunction|FindDifference (Variables|Algo|GetPlayersByTeam)))
    (Variables|Algo|SetAdvantageWinningTeam _difference)
    (else
      (Variables|Algo|SetCurrentWinningTeam 0))))

(event Custom|TurnOn
  (params (Player :type Light%20Wars%20Player%20Object%20Reference))
  (Utilities|Array|AddUnique (Variables|Algo|GetPlayers) Player)
  (CallFunction|AddTeam (Variables|/Game/LightWarsBP/Blueprints/Model/LightWarsPlayer.LightWarsPlayer_C|GetTeamOwner Player)))

(fn FindDifference
  (params (Array :type Array%20of%20Integers))
  (bind (_indexofmaxvalue _maxvalue) (Math|Integer|MaxOfIntArray Array))
  (LocalVariables|SetMaxElement _maxvalue)
  (LocalVariables|SetMaxIndexElement _indexofmaxvalue)
  (LocalVariables|SetDifferenceTmp (Utilities|Array|Length Array))
  (for (_array_element _array_index) Array
    (if (!= (LocalVariables|GetMaxIndexElement) _array_index)
      (if (> (LocalVariables|GetDifferenceTmp) (- (LocalVariables|GetMaxElement) _array_element))
        (LocalVariables|SetDifferenceTmp (- (LocalVariables|GetMaxElement) _array_element)))))
  (return (LocalVariables|GetDifferenceTmp)))

(fn OnRepTeamOwner
  (Default|UpdateOwnerTeam (Variables|Default|GetObserver) (Variables|Default|GetTeamOwner)))
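; Game mode for LightWars that populates the level with characters and registers new players.
; On BeginPlay it finds every SpawnZone actor and spawns an AI LightWarsCharacter at each one's location and rotation, with debug prints around the setup.
; A NotifyNewPlayer event hands each new player to LightWarsGameState through AddPlayer.
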(event `self.ReceiveBeginPlay`
  (`KismetSystemLibrary.PrintString` "GameMode Init running")
  (bind _outactors (`GameplayStatics.GetAllActorsOfClass` "/Game/LightWarsBP/Blueprints/UE4View/SpawnZone.SpawnZone_C"))
  (for _array_element _outactors
    (`AIBlueprintHelperLibrary.SpawnAIFromClass` "/Game/LightWarsBP/Blueprints/UE4View/LightWarsCharacter.LightWarsCharacter_C" null (.location (`self.GetTransform` _array_element)) (.rotation (`self.GetTransform` _array_element))))
  (`KismetSystemLibrary.PrintString` "GameMode Init Success"))

(event `NotifyNewPlayer`
  (params (NewPlayer :type "/Game/LightWarsBP/Blueprints/Model/LightWarsPlayer Object Reference"))
  (bind _aslight_wars_game_state (cast `/Game/LightWarsBP/Blueprints/UE4Model/LightWarsGameState` (`GameplayStatics.GetGameState`)))
  (`/Game/LightWarsBP/Blueprints/UE4Model/LightWarsGameState.AddPlayer` _aslight_wars_game_state NewPlayer))

(fn `UserConstructionScript`)
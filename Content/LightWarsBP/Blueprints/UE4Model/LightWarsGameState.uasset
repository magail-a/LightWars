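; LightWarsGameState is the game state Blueprint for LightWars, owning the Level object and passing new players to it.
; CreateLevel lazily constructs Level with the game state as Outer and calls its Init, only when none exists yet.
; Both BeginPlay and AddPlayer call CreateLevel, so a Level exists before AddPlayer forwards the player, whichever event fires first.
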(event `self.ReceiveBeginPlay`
  (`self.CreateLevel`))

(event `self.ReceiveTick`
  (params (DeltaSeconds :type "Float (single-precision)")))

(event `AddPlayer`
  (params (NewPlayer :type "/Game/LightWarsBP/Blueprints/Model/LightWarsPlayer Object Reference"))
  (`self.CreateLevel`)
  (`/Game/LightWarsBP/Blueprints/Model/Level.AddPlayer` (`self.Level`) NewPlayer))

(event `CreateLevel`
  (if (== (`self.Level`) null)
    (bind _returnvalue (`|GenericCreateObject` "/Game/LightWarsBP/Blueprints/Model/Level.Level_C" self))
    (bind _output_get (set `self.Level` _returnvalue))
    (`/Game/LightWarsBP/Blueprints/Model/Level.Init` _output_get)))

(fn `UserConstructionScript`)
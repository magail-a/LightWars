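; Level model for LightWars that holds the match's teams and players.
; Init constructs a fixed number of Team objects and gives each a color from a color array.
; AddPlayer registers each new player, links it with a team in both directions, and advances a wrapping index to spread players across teams round-robin.
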(event `Init`
  (for _index (range 1 (+ (`self.NB_TEAM`) 1))
    (bind _returnvalue (`|GenericCreateObject` "/Game/LightWarsBP/Blueprints/Model/Team.Team_C" "/Game/LightWarsBP/Blueprints/Model/Team.Team_C"))
    (`KismetArrayLibrary.Array_Add` (`self.Teams`) _returnvalue)
    (set `/Game/LightWarsBP/Blueprints/Model/Team.Color` (`KismetArrayLibrary.Array_Get` (`self.Color`) (- _index 1)) _returnvalue)))

(event `AddPlayer`
  (params (NewPlayer :type "/Game/LightWarsBP/Blueprints/Model/LightWarsPlayer Object Reference"))
  (bind _indexlastteam (`self.IndexLastTeam`))
  (bind _item (`KismetArrayLibrary.Array_Get` (`self.Teams`) _indexlastteam))
  (`KismetArrayLibrary.Array_Add` (`self.Players`) NewPlayer)
  (`KismetArrayLibrary.Array_Add` (`/Game/LightWarsBP/Blueprints/Model/Team.Players` _item) NewPlayer)
  (set `/Game/LightWarsBP/Blueprints/Model/LightWarsPlayer.TeamOwner` _item NewPlayer)
  (bind _result (`/Engine/EditorBlueprintResources/StandardMacros.IncrementInt` _indexlastteam)
    (:`  `
      (set `self.IndexLastTeam` (mod _result (`KismetArrayLibrary.Array_Length` (`self.Teams`)))))))
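; LightWarsCharacterView is the Unreal-side view of a Light Wars character, paired with a LightWarsCharacterController that it creates, ticks and notifies of generator zone entry and exit.
; Team updates recolor the pawn and player light bar, while light updates adjust the bar and destroy the pawn at zero.
; Pawn destruction requests a GameMode respawn delay, then a new character spawns at a fixed transform with light restored and rebinds the destroy event.
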(event `Initialize`
  ;[1 1 1] Init
  (bind _returnvalue (`|GenericCreateObject` "/Game/LightWarsBP/Blueprints/UE4Controller/LightWarsCharacterController.LightWarsCharacterController_C" self (`self.Gamemode`)))
  (bind _output_get (set `self.LightWarsController` _returnvalue))
  (`/Game/LightWarsBP/Blueprints/UE4Controller/LightWarsCharacterController.Init` _output_get self)
  (`self.BindRespawn`))

(event `BindRespawn`
  ;[1 1 1] Respawn
  (add `Actor.OnDestroyed` (`Controller.K2_GetPawn` (`self.UnrealController`)) (delegate `RespawnOnDetroyed`)))

(event `OnSpawDelayExpiration`
  ;[1 1 1] Respawn
  (`self.ResetValues`)
  (bind _transform (`self.GetSpawnTransform`))
  (bind (_character _newcontroller) (`/Game/LightWarsBP/Blueprints/UE4Controller/LightWarsGameMode.SpawnCharacter` (`self.Gamemode`) self _transform))
  (set `self.UnrealController` _newcontroller)
  (set `/Game/LightWarsBP/Blueprints/UE4View/LightWarsCharacter.LightWarsCharacterView` self _character)
  (`self.InitializeCharacter`)
  (`self.BindRespawn`))

(event `RespawnOnDetroyed`
  ;[1 1 1] Respawn
  (`/Game/LightWarsBP/Blueprints/UE4Controller/LightWarsGameMode.RespawnDelay` (`self.Gamemode`) self))

(event `Tick`
  (params (Delta :type "Float (double-precision)"))
  ;[1 1 1] Tick
  (`/Game/LightWarsBP/Blueprints/UE4Controller/LightWarsCharacterController.Tick` (`self.LightWarsController`) Delta))

(event `/Game/LightWarsBP/Blueprints/Model/PlayerObserver.UpdateTeam`
  (params (Team :type "/Game/LightWarsBP/Blueprints/Model/Team Object Reference"))
  ;[1 1 1] Update Team
  (`KismetSystemLibrary.PrintString` null "Event Update Team")
  (`|ExecutionSequence`
    (:`then_0`
      (bind _aslight_wars_player_controller (cast `/Game/LightWarsBP/Blueprints/UE4View/LightWarsPlayerController` (`self.UnrealController`)))
      (`/Game/LightWarsBP/Blueprints/UE4View/LightWarsPlayerController.ChangeLightBarColor` _aslight_wars_player_controller (`/Game/LightWarsBP/Blueprints/Model/Team.Color` Team)))
    (:`then_1`
      (bind _aslight_wars_character (cast `/Game/LightWarsBP/Blueprints/UE4View/LightWarsCharacter` (`Controller.K2_GetPawn` (`self.UnrealController`))))
      (`/Game/LightWarsBP/Blueprints/UE4View/LightWarsCharacter.ChangeColor` _aslight_wars_character (`/Game/LightWarsBP/Blueprints/Model/Team.Color` Team)))))

(event `/Game/LightWarsBP/Blueprints/Model/PlayerObserver.UpdateLight`
  (params (Light :type "Float (single-precision)"))
  ;[1 1 1] Update Light
  (`|ExecutionSequence`
    (:`then_0`
      (bind _aslight_wars_player_controller (cast `/Game/LightWarsBP/Blueprints/UE4View/LightWarsPlayerController` (`self.UnrealController`)))
      (`/Game/LightWarsBP/Blueprints/UE4View/LightWarsPlayerController.UpdateLightBarColor` _aslight_wars_player_controller Light))
    (:`then_1`
      (if (<= Light 0.0)
        (`self.Die`)))))

(event `EnterZone`
  (params (Generator :type "/Game/LightWarsBP/Blueprints/Model/Generator Object Reference"))
  ;[1 1 1] Enter and Exit generator zones
  (`/Game/LightWarsBP/Blueprints/UE4Controller/LightWarsCharacterController.EnterZone` (`self.LightWarsController`) Generator))

(event `ExitZone`
  ;[1 1 1] Enter and Exit generator zones
  (`/Game/LightWarsBP/Blueprints/UE4Controller/LightWarsCharacterController.ExitZone` (`self.LightWarsController`)))

(fn `Die`
  (`Actor.K2_DestroyActor` (`Controller.K2_GetPawn` (`self.UnrealController`))))

(fn `GetSpawnTransform`
  (returns (Transform :type "Transform Structure"))
  (return (`KismetMathLibrary.MakeTransform` (0.0 0.0 1000.0))))

(fn `InitializeCharacter`
  (bind _player (`/Game/LightWarsBP/Blueprints/UE4Controller/LightWarsCharacterController.Player` (`self.LightWarsController`)))
  (set `/Game/LightWarsBP/Blueprints/Model/LightWarsPlayer.Light` 100.0 _player)
  (`/Game/LightWarsBP/Blueprints/Model/LightWarsPlayer.OnRep_TeamOwner` _player))

(fn `ResetValues`)
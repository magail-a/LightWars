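; Light Wars controller that owns a player's Light resource and handles the respawn location.
; Init creates the LightWarsPlayer object, links its observer and notifies the game mode.
; Tick refills Light inside a same-team generator zone, four times faster than it drains otherwise, using the zone set by EnterZone and ExitZone.
; RespawnPlayer picks the nearest team generator, destroys the pawn and resets Light; GetRespawnPlayer returns an offset transform there.
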(event `Init`
  (params (PlayerObserver :type "/Game/LightWarsBP/Blueprints/Model/PlayerObserver Interface"))
  (`KismetSystemLibrary.PrintString` null "Controller Init running")
  (bind _returnvalue (`|GenericCreateObject` "/Game/LightWarsBP/Blueprints/Model/LightWarsPlayer.LightWarsPlayer_C" self 100.0))
  (bind _output_get (set `self.Player` _returnvalue))
  (set `/Game/LightWarsBP/Blueprints/Model/LightWarsPlayer.PlayerObserver` PlayerObserver _output_get)
  (`/Game/LightWarsBP/Blueprints/UE4Controller/LightWarsGameMode.NotifyNewPlayer` (`self.GameMode`) _output_get))

(event `Tick`
  (params (delta :type "Float (double-precision)"))
  (bind _player (`self.Player`))
  (bind _player_2 (`self.Player`))
  (if (== (`/Game/LightWarsBP/Blueprints/Model/Generator.TeamOwner` (`self.GeneratorZone`)) (`/Game/LightWarsBP/Blueprints/Model/LightWarsPlayer.TeamOwner` (`self.Player`)))
    (set `/Game/LightWarsBP/Blueprints/Model/LightWarsPlayer.Light` (`KismetMathLibrary.FClamp` (+ (* delta (`self.FACTOR_TIME`) 4.0) (`/Game/LightWarsBP/Blueprints/Model/LightWarsPlayer.Light` _player)) 0.0 100.0) _player)
    (else
      (set `/Game/LightWarsBP/Blueprints/Model/LightWarsPlayer.Light` (`KismetMathLibrary.FClamp` (- (`/Game/LightWarsBP/Blueprints/Model/LightWarsPlayer.Light` _player_2) (* delta (`self.FACTOR_TIME`))) 0.0 100.0) _player_2))))

(event `EnterZone`
  (params (Generator :type "/Game/LightWarsBP/Blueprints/Model/Generator Object Reference"))
  (set `self.GeneratorZone` Generator))

(event `ExitZone`
  (params (Generator :type "/Game/LightWarsBP/Blueprints/Model/Generator Object Reference"))
  (set `self.GeneratorZone` null))

(event `RespawnPlayer`
  (params (Pawn :type "Pawn Object Reference") (Generators :type "Array of /Game/LightWarsBP/Blueprints/UE4View/LightWarsGenerator Object Reference"))
  (set `self.NearGenerator` null)
  (set `self.MinDistance` 10000000000000.0)
  (for _array_element Generators
    (if (== (`/Game/LightWarsBP/Blueprints/Model/Generator.TeamOwner` (`/Game/LightWarsBP/Blueprints/UE4View/LightWarsGenerator.Generator` _array_element)) (`/Game/LightWarsBP/Blueprints/Model/LightWarsPlayer.TeamOwner` (`self.Player`)))
      (bind _returnvalue (`KismetMathLibrary.VSize` (- (`Actor.K2_GetActorLocation` Pawn) (`Actor.K2_GetActorLocation` _array_element))))
      (if (> (`self.MinDistance`) _returnvalue)
        (set `self.MinDistance` _returnvalue)
        (set `self.NearGenerator` _array_element))))
  (`Actor.K2_DestroyActor` Pawn)
  (set `/Game/LightWarsBP/Blueprints/Model/LightWarsPlayer.Light` 100.0 (`self.Player`)))

(fn `GetRespawnPlayer`
  (returns (Transform :type "Transform Structure"))
  (return (`KismetMathLibrary.MakeTransform` (`KismetMathLibrary.MakeVector` (+ (.x (.location (`Actor.GetTransform` (`self.NearGenerator`)))) 100.0) (.y (.location (`Actor.GetTransform` (`self.NearGenerator`)))) (+ (.z (.location (`Actor.GetTransform` (`self.NearGenerator`)))) 200.0)) (.rotation (`Actor.GetTransform` (`self.NearGenerator`))) (.scale (`Actor.GetTransform` (`self.NearGenerator`))))))
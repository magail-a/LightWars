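; Capturable generator actor in LightWars: it acts as the world view of a Generator object, which it creates, ticks and observes.
; On BeginPlay it also spawns a companion generator zone.
; Overlapping characters start or stop capture for their player, while a widget shows capture progress in the previous winning team's color.
; On owner team updates, dynamic glass materials tint the capture and zone cylinders, or black when unowned.
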(event `self.ReceiveBeginPlay`
  (bind _returnvalue (`|GenericCreateObject` "/Game/LightWarsBP/Blueprints/Model/Generator.Generator_C" self))
  (bind _output_get (set `self.Generator` _returnvalue))
  (set `/Game/LightWarsBP/Blueprints/Model/Generator.Observer` self _output_get)
  (bind _returnvalue_2 (`|SpawnActorFromClass` "/Game/LightWarsBP/Blueprints/UE4View/LightWarsGeneratorZone.LightWarsGeneratorZone_C" (`self.GetTransform`) "AlwaysSpawn" "OverrideRootScale" null self))
  (set `self.Zone` _returnvalue_2))

(event `self.ReceiveActorBeginOverlap`
  (params (OtherActor :type "Actor Object Reference"))
  (bind _aslight_wars_character (cast `/Game/LightWarsBP/Blueprints/UE4View/LightWarsCharacter` OtherActor))
  (`/Game/LightWarsBP/Blueprints/Model/Generator.TurnOn` (`self.Generator`) (`/Game/LightWarsBP/Blueprints/UE4Controller/LightWarsCharacterController.Player` (`/Game/LightWarsBP/Blueprints/UE4View/LightWarsCharacterView.LightWarsController` (`/Game/LightWarsBP/Blueprints/UE4View/LightWarsCharacter.LightWarsCharacterView` _aslight_wars_character)))))

(event `self.ReceiveActorEndOverlap`
  (params (OtherActor :type "Actor Object Reference"))
  (bind _aslight_wars_character (cast `/Game/LightWarsBP/Blueprints/UE4View/LightWarsCharacter` OtherActor))
  (`/Game/LightWarsBP/Blueprints/Model/Generator.StopTurnOn` (`self.Generator`) (`/Game/LightWarsBP/Blueprints/UE4Controller/LightWarsCharacterController.Player` (`/Game/LightWarsBP/Blueprints/UE4View/LightWarsCharacterView.LightWarsController` (`/Game/LightWarsBP/Blueprints/UE4View/LightWarsCharacter.LightWarsCharacterView` _aslight_wars_character)))))

(event `self.ReceiveTick`
  (params (DeltaSeconds :type "Float (single-precision)"))
  (bind _generator (`self.Generator`))
  (bind _previouswinningteam (`/Game/LightWarsBP/Blueprints/Model/Generator.PreviousWinningTeam` _generator))
  (`|ExecutionSequence`
    (:`then_0`
      (`/Game/LightWarsBP/Blueprints/Model/Generator.Tick` (`self.Generator`) DeltaSeconds))
    (:`then_1`
      (bind _asprogress_generator (cast `/Game/LightWarsBP/Blueprints/UE4View/HUD/ProgressGenerator` (`WidgetComponent.GetUserWidgetObject` (`self.Progress`))))
      (bind _progress (`/Game/LightWarsBP/Blueprints/UE4View/HUD/ProgressGenerator.Progress` _asprogress_generator))
      (`ProgressBar.SetPercent` _progress (/ (`/Game/LightWarsBP/Blueprints/Model/Generator.ProgressCapture` _generator) 100.0))
      (`/Engine/EditorBlueprintResources/StandardMacros.IsValid` _previouswinningteam
        (:`Is Valid`
          (`ProgressBar.SetFillColorAndOpacity` _progress (`/Game/LightWarsBP/Blueprints/Model/Team.Color` _previouswinningteam)))))))

(event `/Game/LightWarsBP/Blueprints/Model/GeneratorObserver.UpdateOwnerTeam`
  (params (OwnerTeam :type "/Game/LightWarsBP/Blueprints/Model/Team Object Reference"))
  (if (== OwnerTeam null)
    (bind _returnvalue (`KismetMaterialLibrary.CreateDynamicMaterialInstance` "/Game/StarterContent/Materials/M_GlassInstance.M_GlassInstance"))
    (`MaterialInstanceDynamic.SetVectorParameterValue` :`self` _returnvalue :`ParameterName` "ColorGlass")
    (`PrimitiveComponent.SetMaterial` (`self.CylinderCapture`) 0 _returnvalue)
    (`PrimitiveComponent.SetMaterial` (`/Game/LightWarsBP/Blueprints/UE4View/LightWarsGeneratorZone.CylinderLimit` (`self.Zone`)) 0 _returnvalue)
    (else
      (bind _returnvalue_2 (`KismetMaterialLibrary.CreateDynamicMaterialInstance` "/Game/StarterContent/Materials/M_GlassInstance.M_GlassInstance"))
      (`MaterialInstanceDynamic.SetVectorParameterValue` _returnvalue_2 "ColorGlass" (`/Game/LightWarsBP/Blueprints/Model/Team.Color` OwnerTeam))
      (`PrimitiveComponent.SetMaterial` (`self.CylinderCapture`) 0 _returnvalue_2)
      (`PrimitiveComponent.SetMaterial` (`/Game/LightWarsBP/Blueprints/UE4View/LightWarsGeneratorZone.CylinderLimit` (`self.Zone`)) 0 _returnvalue_2))))

(fn `UserConstructionScript`)